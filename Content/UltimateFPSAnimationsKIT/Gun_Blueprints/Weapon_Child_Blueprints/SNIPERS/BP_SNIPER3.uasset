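; BP_SNIPER3 is a child weapon Blueprint for a five-round, manually cycled FPS sniper rifle.
; Fire alternates shooting and chambering, using a spread-randomized camera trace to place a decal and aim a projectile spawned at the muzzle.
; Reload loops single-round insertions until full, with montage lengths timing each phase and separate hip and ADS arm animations.
; SniperZoom lerps FOV and removes spread; undrawing saves weapon state to the player.
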(event Custom|Draw
  ;[1 1 1] Draw
  (Utilities|DrawMacro))

(event Custom|Undraw
  ;[1 1 1] Undraw
  (bind _returnvalue (Utilities|UndrawMacro)
    (:Completed
      (Variables|Default|SetUndrawTime _returnvalue))))

(event EventReload
  (bind _returnvalue (Game|GetPlayerCharacter 0))
  (bind _returnvalue_2 (Game|GetPlayerCharacter 0))
  (bind _returnvalue_3 (Game|GetPlayerCharacter 0))
  (bind _primaryweapon (Variables|Default|GetPrimaryWeapon))
  (bind _primaryweapon_2 (Variables|Default|GetPrimaryWeapon))
  (bind _asbp_player_character (Utilities|Casting|CastToBP_PlayerCharacter _returnvalue_2))
  (bind _asbp_player_character_2 (Utilities|Casting|CastToBP_PlayerCharacter _returnvalue))
  (bind _asbp_player_character_3 (Utilities|Casting|CastToBP_PlayerCharacter _returnvalue_3))
  (bind _arms (Variables|/Game/UltimateFPSAnimationsKIT/Demo/PlayerMannequin/BP_PlayerCharacter.BP_PlayerCharacter_C|GetArms _asbp_player_character))
  (bind _returnvalue_4 (Components|SkeletalMesh|GetAnimInstance _arms))
  ;[1 1 1] Reload
  (if (< (Variables|Default|GetAmmoCount) (Variables|Default|GetMaxAmmo))
    (if (Variables|/Game/UltimateFPSAnimationsKIT/Demo/PlayerMannequin/BP_PlayerCharacter.BP_PlayerCharacter_C|GetAimDownSight _asbp_player_character)
      (Variables|/Game/UltimateFPSAnimationsKIT/Demo/PlayerMannequin/BP_PlayerCharacter.BP_PlayerCharacter_C|SetIsReloading _asbp_player_character true)
      (Utilities|FlowControl|Sequence
        (:then_0
          (bind _returnvalue_5 (Animation|Montage|MontagePlay _returnvalue_4 "/Game/UltimateFPSAnimationsKIT/Animations/Arms_Montages/SNIPER3_arms_reload_phase_1_ads_Montage.SNIPER3_arms_reload_phase_1_ads_Montage" 1.0 "MontageLength" 0.0 true))
          (Components|Animation|PlayAnimation _primaryweapon "/Game/UltimateFPSAnimationsKIT/Animations/Gun/SNIPER3_gun_reload_phase_1.SNIPER3_gun_reload_phase_1" false)
          (Utilities|FlowControl|Delay _returnvalue_5)
          (Variables|/Game/UltimateFPSAnimationsKIT/Demo/PlayerMannequin/BP_PlayerCharacter.BP_PlayerCharacter_C|SetIsReloading _asbp_player_character false)
          (Variables|/Game/UltimateFPSAnimationsKIT/Demo/PlayerMannequin/BP_PlayerCharacter.BP_PlayerCharacter_C|SetIsReloading _asbp_player_character true :!label _label)
          (bind _returnvalue_6 (Animation|Montage|MontagePlay _returnvalue_4 "/Game/UltimateFPSAnimationsKIT/Animations/Arms_Montages/SNIPER3_arms_reload_phase_2_ads_Montage.SNIPER3_arms_reload_phase_2_ads_Montage" 1.0 "MontageLength" 0.0 true))
          (Components|Animation|PlayAnimation _primaryweapon "/Game/UltimateFPSAnimationsKIT/Animations/Gun/SNIPER3_gun_reload_phase_2.SNIPER3_gun_reload_phase_2" false)
          (CallFunction|UnHideBullets)
          (Utilities|FlowControl|Delay _returnvalue_6)
          (Variables|Default|SetAmmoCount (+ (Variables|Default|GetAmmoCount) 1))
          (Variables|/Game/UltimateFPSAnimationsKIT/Demo/PlayerMannequin/BP_PlayerCharacter.BP_PlayerCharacter_C|SetIsReloading _asbp_player_character_2 false)
          (CallFunction|HideBullets)
          (if (== (Variables|Default|GetAmmoCount) (Variables|Default|GetMaxAmmo))
            (Variables|/Game/UltimateFPSAnimationsKIT/Demo/PlayerMannequin/BP_PlayerCharacter.BP_PlayerCharacter_C|SetIsReloading _asbp_player_character_2 true)
            (bind _returnvalue_7 (Animation|Montage|MontagePlay (Components|SkeletalMesh|GetAnimInstance (Variables|/Game/UltimateFPSAnimationsKIT/Demo/PlayerMannequin/BP_PlayerCharacter.BP_PlayerCharacter_C|GetArms _asbp_player_character_2)) "/Game/UltimateFPSAnimationsKIT/Animations/Arms_Montages/SNIPER3_arms_reload_phase_3ads_Montage.SNIPER3_arms_reload_phase_3ads_Montage" 1.0 "MontageLength" 0.0 true))
            (Components|Animation|PlayAnimation (Variables|Default|GetPrimaryWeapon) "/Game/UltimateFPSAnimationsKIT/Animations/Gun/SNIPER3_gun_reload_phase_3.SNIPER3_gun_reload_phase_3" false)
            (Utilities|FlowControl|Delay _returnvalue_7)
            (Variables|/Game/UltimateFPSAnimationsKIT/Demo/PlayerMannequin/BP_PlayerCharacter.BP_PlayerCharacter_C|SetIsReloading _asbp_player_character_2 false)
            (Variables|Default|SetChamberedAmmo true)
            (else
              (goto _label))))
        (:then_1
          (if (not (Variables|Default|GetChamberedAmmo))
            (Utilities|FlowControl|Delay 0.5)
            (Utilities|EjectShell))))
      (else
        (Variables|/Game/UltimateFPSAnimationsKIT/Demo/PlayerMannequin/BP_PlayerCharacter.BP_PlayerCharacter_C|SetIsReloading _asbp_player_character true)
        (Utilities|FlowControl|Sequence
          (:then_0
            (bind _returnvalue_8 (Animation|Montage|MontagePlay _returnvalue_4 "/Game/UltimateFPSAnimationsKIT/Animations/Arms_Montages/SNIPER3_arms_reload_phase_1_Montage.SNIPER3_arms_reload_phase_1_Montage" 1.0 "MontageLength" 0.0 true))
            (Components|Animation|PlayAnimation _primaryweapon_2 "/Game/UltimateFPSAnimationsKIT/Animations/Gun/SNIPER3_gun_reload_phase_1.SNIPER3_gun_reload_phase_1" false)
            (Utilities|FlowControl|Delay _returnvalue_8)
            (Variables|/Game/UltimateFPSAnimationsKIT/Demo/PlayerMannequin/BP_PlayerCharacter.BP_PlayerCharacter_C|SetIsReloading _asbp_player_character false)
            (Variables|/Game/UltimateFPSAnimationsKIT/Demo/PlayerMannequin/BP_PlayerCharacter.BP_PlayerCharacter_C|SetIsReloading _asbp_player_character true :!label _label_2)
            (bind _returnvalue_9 (Animation|Montage|MontagePlay _returnvalue_4 "/Game/UltimateFPSAnimationsKIT/Animations/Arms_Montages/SNIPER3_arms_reload_phase_2_Montage.SNIPER3_arms_reload_phase_2_Montage" 1.0 "MontageLength" 0.0 true))
            (CallFunction|UnHideBullets)
            (Components|Animation|PlayAnimation _primaryweapon_2 "/Game/UltimateFPSAnimationsKIT/Animations/Gun/SNIPER3_gun_reload_phase_2.SNIPER3_gun_reload_phase_2" false)
            (Utilities|FlowControl|Delay _returnvalue_9)
            (Variables|Default|SetAmmoCount (+ (Variables|Default|GetAmmoCount) 1))
            (Variables|/Game/UltimateFPSAnimationsKIT/Demo/PlayerMannequin/BP_PlayerCharacter.BP_PlayerCharacter_C|SetIsReloading _asbp_player_character_3 false)
            (CallFunction|HideBullets)
            (if (== (Variables|Default|GetAmmoCount) (Variables|Default|GetMaxAmmo))
              (Variables|/Game/UltimateFPSAnimationsKIT/Demo/PlayerMannequin/BP_PlayerCharacter.BP_PlayerCharacter_C|SetIsReloading _asbp_player_character_3 true)
              (bind _returnvalue_10 (Animation|Montage|MontagePlay (Components|SkeletalMesh|GetAnimInstance (Variables|/Game/UltimateFPSAnimationsKIT/Demo/PlayerMannequin/BP_PlayerCharacter.BP_PlayerCharacter_C|GetArms _asbp_player_character_3)) "/Game/UltimateFPSAnimationsKIT/Animations/Arms_Montages/SNIPER3_arms_reload_phase_3_Montage.SNIPER3_arms_reload_phase_3_Montage" 1.0 "MontageLength" 0.0 true))
              (Components|Animation|PlayAnimation (Variables|Default|GetPrimaryWeapon) "/Game/UltimateFPSAnimationsKIT/Animations/Gun/SNIPER3_gun_reload_phase_3.SNIPER3_gun_reload_phase_3" false)
              (Utilities|FlowControl|Delay _returnvalue_10)
              (Variables|/Game/UltimateFPSAnimationsKIT/Demo/PlayerMannequin/BP_PlayerCharacter.BP_PlayerCharacter_C|SetIsReloading _asbp_player_character_3 false)
              (Variables|Default|SetChamberedAmmo true)
              (else
                (goto _label_2))))
          (:then_1
            (if (not (Variables|Default|GetChamberedAmmo))
              (Utilities|FlowControl|Delay 0.5)
              (Utilities|EjectShell))))))))

(event EventHideMuzzleFlash
  ;[1 1 1] Hide/UnhideMuzzleflash
  (Rendering|Material|SetMaterial (Variables|Default|GetMuzzelFlashPlane) 0 "/Game/UltimateFPSAnimationsKIT/GunModels/Materials/M_Transparent.M_Transparent")
  (Rendering|SetVisibility (Variables|Default|GetPointLight) false false))

(event EventFire
  (bind _returnvalue (Game|GetPlayerCharacter 0))
  (bind _returnvalue_2 (Game|GetPlayerCharacter 0))
  (bind _asbp_player_character (Utilities|Casting|CastToBP_PlayerCharacter _returnvalue_2))
  (bind _asbp_player_character_2 (Utilities|Casting|CastToBP_PlayerCharacter _returnvalue))
  (bind _arms (Variables|/Game/UltimateFPSAnimationsKIT/Demo/PlayerMannequin/BP_PlayerCharacter.BP_PlayerCharacter_C|GetArms _asbp_player_character))
  (bind _arms_2 (Variables|/Game/UltimateFPSAnimationsKIT/Demo/PlayerMannequin/BP_PlayerCharacter.BP_PlayerCharacter_C|GetArms _asbp_player_character_2))
  (bind _returnvalue_3 (Components|SkeletalMesh|GetAnimInstance _arms_2))
  ;[1 1 1] Fire
  (if (Variables|Default|GetChamberedAmmo)
    (Variables|Default|SetChamberedAmmo false)
    (if (> (Variables|Default|GetAmmoCount) 0)
      (CallFunction|AmmoCheck)
      (Default|IncreaseSpread (.AsBP%20Player%20Character (Utilities|Casting|CastToBP_PlayerCharacter (Game|GetPlayerCharacter 0))) 1.0)
      (bind (_muzzlelocation _impactpoint _projectilerotation) (CallFunction|LineTrace))
      (CallFunction|SpawnBulletProjectile _muzzlelocation _impactpoint _impactpoint _projectilerotation)
      (if (Variables|/Game/UltimateFPSAnimationsKIT/Demo/PlayerMannequin/BP_PlayerCharacter.BP_PlayerCharacter_C|GetAimDownSight _asbp_player_character)
        (Animation|Montage|PlayMontage _arms "/Game/UltimateFPSAnimationsKIT/Animations/Arms_Montages/SNIPER3_arms_fire_ads_Montage.SNIPER3_arms_fire_ads_Montage"
          (:then
            _))
        (else
          (Animation|Montage|PlayMontage _arms "/Game/UltimateFPSAnimationsKIT/Animations/Arms_Montages/SNIPER3_arms_fire_Montage.SNIPER3_arms_fire_Montage"
            (:then
              _))))
      (Utilities|MuzzleFlash)
      (Audio|PlaySound2D "/Game/UltimateFPSAnimationsKIT/SoundFX/gunshot7.gunshot7" 1.0 1.0 0.0 0 0)
      (Game|Feedback|ClientStartCameraShake (Game|GetPlayerController 0) "/Game/UltimateFPSAnimationsKIT/CameraShake/BP_CameraShake_Mega.BP_CameraShake_Mega_C" 1.0 "CameraLocal" "0, 0, 0")
      (else
        (Audio|PlaySound2D "/Game/UltimateFPSAnimationsKIT/SoundFX/dryfire.dryfire" 1.0 1.0 0.0 0 0)))
    (elif (> (Variables|Default|GetAmmoCount) 0)
      (Variables|/Game/UltimateFPSAnimationsKIT/Demo/PlayerMannequin/BP_PlayerCharacter.BP_PlayerCharacter_C|SetIsReloading _asbp_player_character_2 true)
      ;[1 1 1] Chamber New  Round
      (if (Variables|/Game/UltimateFPSAnimationsKIT/Demo/PlayerMannequin/BP_PlayerCharacter.BP_PlayerCharacter_C|GetAimDownSight _asbp_player_character_2)
        (bind _returnvalue_4 (Animation|Montage|MontagePlay _returnvalue_3 "/Game/UltimateFPSAnimationsKIT/Animations/Arms_Montages/SNIPER3_arms_chamber_ads_Montage.SNIPER3_arms_chamber_ads_Montage" 1.0 "MontageLength" 0.0 true))
        (Components|Animation|PlayAnimation (Variables|Default|GetPrimaryWeapon) "/Game/UltimateFPSAnimationsKIT/Animations/Gun/SNIPER3_gun_chamber.SNIPER3_gun_chamber" false)
        (Utilities|FlowControl|Sequence
          (:then_0
            (Utilities|FlowControl|Delay _returnvalue_4)
            (Variables|Default|SetChamberedAmmo true)
            (Variables|/Game/UltimateFPSAnimationsKIT/Demo/PlayerMannequin/BP_PlayerCharacter.BP_PlayerCharacter_C|SetIsReloading _asbp_player_character_2 false))
          (:then_1
            (Utilities|FlowControl|Delay 0.5)
            (Utilities|EjectShell)))
        (else
          (bind _returnvalue_5 (Animation|Montage|MontagePlay _returnvalue_3 "/Game/UltimateFPSAnimationsKIT/Animations/Arms_Montages/SNIPER3_arms_chamber_Montage.SNIPER3_arms_chamber_Montage" 1.0 "MontageLength" 0.0 true))
          (Components|Animation|PlayAnimation (Variables|Default|GetPrimaryWeapon) "/Game/UltimateFPSAnimationsKIT/Animations/Gun/SNIPER3_gun_chamber.SNIPER3_gun_chamber" false)
          (Utilities|FlowControl|Sequence
            (:then_0
              (Utilities|FlowControl|Delay _returnvalue_5)
              (Variables|Default|SetChamberedAmmo true)
              (Variables|/Game/UltimateFPSAnimationsKIT/Demo/PlayerMannequin/BP_PlayerCharacter.BP_PlayerCharacter_C|SetIsReloading _asbp_player_character_2 false))
            (:then_1
              (Utilities|FlowControl|Delay 0.5)
              (Utilities|EjectShell))))))))

(event EventUnhideMuzzleFlash
  ;[1 1 1] Hide/UnhideMuzzleflash
  (Rendering|Material|SetMaterial (Variables|Default|GetMuzzelFlashPlane) 0 "/Game/UltimateFPSAnimationsKIT/TexturesAndMats/M_MuzzleFlash.M_MuzzleFlash")
  (Rendering|SetVisibility (Variables|Default|GetPointLight) true false))

(event EventEquipe
  (bind _returnvalue (Game|GetPlayerCharacter 0))
  (bind _asbp_player_character (Utilities|Casting|CastToBP_PlayerCharacter _returnvalue))
  ;[1 1 1] Equipe
  (Animation|Montage|MontagePlay (Components|SkeletalMesh|GetAnimInstance (Variables|/Game/UltimateFPSAnimationsKIT/Demo/PlayerMannequin/BP_PlayerCharacter.BP_PlayerCharacter_C|GetArms _asbp_player_character)) "/Game/UltimateFPSAnimationsKIT/Animations/Arms_Montages/SNIPER3_arms_equipe_Montage.SNIPER3_arms_equipe_Montage" 1.0 "MontageLength" 0.0 true)
  (Components|Animation|PlayAnimation (Variables|Default|GetPrimaryWeapon) "/Game/UltimateFPSAnimationsKIT/Animations/Gun/SNIPER3_gun_equipe.SNIPER3_gun_equipe" false)
  (Variables|/Game/UltimateFPSAnimationsKIT/Demo/PlayerMannequin/BP_PlayerCharacter.BP_PlayerCharacter_C|SetKnifeActive _asbp_player_character false))

(event EventSniperZoom
  (params (Toggle :type Boolean))
  (bind _returnvalue (Game|GetPlayerCharacter 0))
  (bind _asbp_player_character (Utilities|Casting|CastToBP_PlayerCharacter _returnvalue))
  (bind _playercamera (Variables|/Game/UltimateFPSAnimationsKIT/Demo/PlayerMannequin/BP_PlayerCharacter.BP_PlayerCharacter_C|GetPlayerCamera _asbp_player_character))
  ;[1 1 1] Sniper Zoom FOV Change
  (if Toggle
    (bind _float (Timeline|Timeline_0 PlayFromStart)
      (:Update
        (Camera|SetFieldOfView _playercamera (Math|Float|Lerp 9e+01 4e+01 _float))
        (Variables|Default|SetBulletSpread 0.0)))
    (else
      (bind _float_2 (Timeline|Timeline_1 PlayFromStart)
        (:Update
          (Camera|SetFieldOfView _playercamera (Math|Float|Lerp 4e+01 9e+01 _float_2))
          (Variables|Default|SetBulletSpread 5e+02))))))

(event EventBeginPlay
  ;[1 1 1] Hide Bullets
  (CallFunction|HideBullets))

(fn ConstructionScript
  (|CallParentFunction)
  (Variables|Default|SetMaxAmmo 5)
  (Variables|Default|SetAmmoCount 5)
  (Variables|Default|SetReloadTime 2.0)
  (Variables|Default|SetBulletSpread 5e+02)
  (Variables|Default|SetName "NewEnumerator4")
  (Variables|Default|SetVariableMode false))

(fn AmmoCheck
  (Math|Integer|DecrementInt (Variables|Default|GetAmmoCount)
    (:%20%20
      (if (not (Variables|/Game/UltimateFPSAnimationsKIT/Demo/PlayerMannequin/BP_PlayerCharacter.BP_PlayerCharacter_C|GetIsReloading (.AsBP%20Player%20Character (Utilities|Casting|CastToBP_PlayerCharacter (Game|GetPlayerCharacter 0)))))
        (Components|Animation|PlayAnimation (Variables|Default|GetPrimaryWeapon) "/Game/UltimateFPSAnimationsKIT/Animations/Gun/RIFLE1_gun_fire.RIFLE1_gun_fire" false)))))

(fn LineTrace
  (bind _returnvalue (Game|GetPlayerCharacter 0))
  (bind _bulletspread (Variables|Default|GetBulletSpread))
  (bind _muzzle (Variables|Default|GetMuzzle))
  (bind _returnvalue_2 (Transformation|GetWorldLocation _muzzle))
  (bind _asbp_player_character (Utilities|Casting|CastToBP_PlayerCharacter _returnvalue))
  (bind _returnvalue_3 (* _bulletspread -1.0))
  (bind _playercamera (Variables|/Game/UltimateFPSAnimationsKIT/Demo/PlayerMannequin/BP_PlayerCharacter.BP_PlayerCharacter_C|GetPlayerCamera _asbp_player_character))
  (bind _returnvalue_4 (Transformation|GetWorldLocation _playercamera))
  (bind _outhit (Collision|LineTraceByChannel _returnvalue_4 (+ (+ (* (Math|Vector|GetForwardVector _playercamera) 2e+04) _returnvalue_4) (Math|Vector|MakeVector (Math|Random|RandomFloatinRange _returnvalue_3 _bulletspread) (Math|Random|RandomFloatinRange _returnvalue_3 _bulletspread) (Math|Random|RandomFloatinRange _returnvalue_3 _bulletspread))) "TraceTypeQuery1" false 0 "None")) ; CameraLineTrace
  (Collision|LineTraceByChannel _returnvalue_2 (.ImpactPoint (Collision|BreakHitResult _outhit)) "TraceTypeQuery1" false 0 "None" true "(R=0.000000,G=1.000000,B=0.110935,A=1.000000)") ; MuzzleLineTrace
  (return _returnvalue_2 (.ImpactPoint (Collision|BreakHitResult _outhit)) (Math|Rotator|FindLookatRotation (.TraceStart (Collision|BreakHitResult _outhit)) (.TraceEnd (Collision|BreakHitResult _outhit)))))

(fn SpawnBulletProjectile
  (params (MuzzleLocation :type Vector) (ImpactPoint :type Vector) (SpawnTransformLocation :type Vector) (ProjectileRotation :type Rotator))
  (Game|SpawnActorfromClass "/Game/UltimateFPSAnimationsKIT/Gun_Blueprints/BP_BulletDecal.BP_BulletDecal_C" (Math|Transform|MakeTransform SpawnTransformLocation (Math|Conversions|RotationFromXVector ImpactPoint) "0.020000,0.020000,0.020000") "Undefined" 0 0)
  (Game|SpawnActorfromClass "/Game/UltimateFPSAnimationsKIT/Gun_Blueprints/BP_Bullet.BP_Bullet_C" (Math|Transform|MakeTransform MuzzleLocation ProjectileRotation "0.080000,0.080000,0.080000") "Undefined" 0 0)
  (return))

(fn HideBullets
  (bind _primaryweapon (Variables|Default|GetPrimaryWeapon))
  (Components|SkinnedMesh|HideBonebyName _primaryweapon "bullet" "PBO_None")
  (Components|SkinnedMesh|HideBonebyName _primaryweapon "bullet-2" "PBO_None")
  (Components|SkinnedMesh|HideBonebyName _primaryweapon "bullet-3" "PBO_None"))

(fn UnHideBullets
  (bind _primaryweapon (Variables|Default|GetPrimaryWeapon))
  (Components|SkinnedMesh|UnHideBonebyName _primaryweapon "bullet")
  (Components|SkinnedMesh|UnHideBonebyName _primaryweapon "bullet-2")
  (Components|SkinnedMesh|UnHideBonebyName _primaryweapon "bullet-3"))