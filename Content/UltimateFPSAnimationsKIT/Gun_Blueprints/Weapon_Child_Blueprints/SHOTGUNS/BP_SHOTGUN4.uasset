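; Pump-action shotgun weapon child Blueprint (SHOTGUN4) for the FPS player character, driving arms montages and gun animations.
; Fire alternates between shooting five spread pellets, via camera traces that spawn bullets and decals, and chambering a round with shell ejection.
; A recoil timeline kicks the view, then reverses with pitch-scaled recovery.
; Reload loops shell-by-shell until full, with hip and ADS variants, and undraw saves weapon state to the player.
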(event Custom|Draw
  ;[1 1 1] Draw
  (Utilities|DrawMacro))

(event Custom|Undraw
  ;[1 1 1] Undraw
  (bind _returnvalue (Utilities|UndrawMacro)
    (:Completed
      (Variables|Default|SetUndrawTime _returnvalue))))

(event EventReload
  (bind _returnvalue (Game|GetPlayerCharacter 0))
  (bind _returnvalue_2 (Game|GetPlayerCharacter 0))
  (bind _returnvalue_3 (Game|GetPlayerCharacter 0))
  (bind _asbp_player_character (Utilities|Casting|CastToBP_PlayerCharacter _returnvalue_2))
  (bind _asbp_player_character_2 (Utilities|Casting|CastToBP_PlayerCharacter _returnvalue))
  (bind _asbp_player_character_3 (Utilities|Casting|CastToBP_PlayerCharacter _returnvalue_3))
  (bind _arms (Variables|/Game/UltimateFPSAnimationsKIT/Demo/PlayerMannequin/BP_PlayerCharacter.BP_PlayerCharacter_C|GetArms _asbp_player_character))
  (bind _returnvalue_4 (Components|SkeletalMesh|GetAnimInstance _arms))
  ;[1 1 1] Reload
  (if (< (Variables|Default|GetAmmoCount) (Variables|Default|GetMaxAmmo))
    (if (Variables|/Game/UltimateFPSAnimationsKIT/Demo/PlayerMannequin/BP_PlayerCharacter.BP_PlayerCharacter_C|GetAimDownSight _asbp_player_character)
      (Variables|/Game/UltimateFPSAnimationsKIT/Demo/PlayerMannequin/BP_PlayerCharacter.BP_PlayerCharacter_C|SetIsReloading _asbp_player_character true)
      (bind _returnvalue_5 (Animation|Montage|MontagePlay _returnvalue_4 "/Game/UltimateFPSAnimationsKIT/Animations/Arms_Montages/SHOTGUN4_arms_reload_phase_1_ads_Montage.SHOTGUN4_arms_reload_phase_1_ads_Montage" 1.0 "MontageLength" 0.0 true))
      (Utilities|FlowControl|Delay _returnvalue_5)
      (Variables|/Game/UltimateFPSAnimationsKIT/Demo/PlayerMannequin/BP_PlayerCharacter.BP_PlayerCharacter_C|SetIsReloading _asbp_player_character false)
      (Variables|/Game/UltimateFPSAnimationsKIT/Demo/PlayerMannequin/BP_PlayerCharacter.BP_PlayerCharacter_C|SetIsReloading _asbp_player_character true :!label _label)
      (bind _returnvalue_6 (Animation|Montage|MontagePlay _returnvalue_4 "/Game/UltimateFPSAnimationsKIT/Animations/Arms_Montages/SHOTGUN4_arms_reload_phase_2_ads_Montage.SHOTGUN4_arms_reload_phase_2_ads_Montage" 1.0 "MontageLength" 0.0 true))
      (Components|Animation|PlayAnimation (Variables|Default|GetPrimaryWeapon) "/Game/UltimateFPSAnimationsKIT/Animations/Gun/SHOTGUN4_gun_reload_phase_2.SHOTGUN4_gun_reload_phase_2" false)
      (CallFunction|UnHideBullets)
      (Utilities|FlowControl|Delay _returnvalue_6)
      (Variables|Default|SetAmmoCount (+ (Variables|Default|GetAmmoCount) 1))
      (Variables|/Game/UltimateFPSAnimationsKIT/Demo/PlayerMannequin/BP_PlayerCharacter.BP_PlayerCharacter_C|SetIsReloading _asbp_player_character_2 false)
      (CallFunction|HideBullets)
      (if (== (Variables|Default|GetAmmoCount) (Variables|Default|GetMaxAmmo))
        (Variables|/Game/UltimateFPSAnimationsKIT/Demo/PlayerMannequin/BP_PlayerCharacter.BP_PlayerCharacter_C|SetIsReloading _asbp_player_character_2 true)
        (bind _returnvalue_7 (Animation|Montage|MontagePlay (Components|SkeletalMesh|GetAnimInstance (Variables|/Game/UltimateFPSAnimationsKIT/Demo/PlayerMannequin/BP_PlayerCharacter.BP_PlayerCharacter_C|GetArms _asbp_player_character_2)) "/Game/UltimateFPSAnimationsKIT/Animations/Arms_Montages/SHOTGUN4_arms_reload_phase_3_ads_Montage.SHOTGUN4_arms_reload_phase_3_ads_Montage" 1.0 "MontageLength" 0.0 true))
        (Utilities|FlowControl|Delay _returnvalue_7)
        (Variables|/Game/UltimateFPSAnimationsKIT/Demo/PlayerMannequin/BP_PlayerCharacter.BP_PlayerCharacter_C|SetIsReloading _asbp_player_character_2 false)
        (else
          (goto _label)))
      (else
        (Variables|/Game/UltimateFPSAnimationsKIT/Demo/PlayerMannequin/BP_PlayerCharacter.BP_PlayerCharacter_C|SetIsReloading _asbp_player_character true)
        (bind _returnvalue_8 (Animation|Montage|MontagePlay _returnvalue_4 "/Game/UltimateFPSAnimationsKIT/Animations/Arms_Montages/SHOTGUN4_arms_reload_phase_1__Montage.SHOTGUN4_arms_reload_phase_1__Montage" 1.0 "MontageLength" 0.0 true))
        (Utilities|FlowControl|Delay _returnvalue_8)
        (Variables|/Game/UltimateFPSAnimationsKIT/Demo/PlayerMannequin/BP_PlayerCharacter.BP_PlayerCharacter_C|SetIsReloading _asbp_player_character false)
        (Variables|/Game/UltimateFPSAnimationsKIT/Demo/PlayerMannequin/BP_PlayerCharacter.BP_PlayerCharacter_C|SetIsReloading _asbp_player_character true :!label _label_2)
        (bind _returnvalue_9 (Animation|Montage|MontagePlay _returnvalue_4 "/Game/UltimateFPSAnimationsKIT/Animations/Arms_Montages/SHOTGUN4_arms_reload_phase_2_Montage.SHOTGUN4_arms_reload_phase_2_Montage" 1.0 "MontageLength" 0.0 true))
        (CallFunction|UnHideBullets)
        (Components|Animation|PlayAnimation (Variables|Default|GetPrimaryWeapon) "/Game/UltimateFPSAnimationsKIT/Animations/Gun/SHOTGUN4_gun_reload_phase_2.SHOTGUN4_gun_reload_phase_2" false)
        (Utilities|FlowControl|Delay _returnvalue_9)
        (Variables|Default|SetAmmoCount (+ (Variables|Default|GetAmmoCount) 1))
        (Variables|/Game/UltimateFPSAnimationsKIT/Demo/PlayerMannequin/BP_PlayerCharacter.BP_PlayerCharacter_C|SetIsReloading _asbp_player_character_3 false)
        (CallFunction|HideBullets)
        (if (== (Variables|Default|GetAmmoCount) (Variables|Default|GetMaxAmmo))
          (Variables|/Game/UltimateFPSAnimationsKIT/Demo/PlayerMannequin/BP_PlayerCharacter.BP_PlayerCharacter_C|SetIsReloading _asbp_player_character_3 true)
          (bind _returnvalue_10 (Animation|Montage|MontagePlay (Components|SkeletalMesh|GetAnimInstance (Variables|/Game/UltimateFPSAnimationsKIT/Demo/PlayerMannequin/BP_PlayerCharacter.BP_PlayerCharacter_C|GetArms _asbp_player_character_3)) "/Game/UltimateFPSAnimationsKIT/Animations/Arms_Montages/SHOTGUN4_arms_reload_phase_3_Montage.SHOTGUN4_arms_reload_phase_3_Montage" 1.0 "MontageLength" 0.0 true))
          (Utilities|FlowControl|Delay _returnvalue_10)
          (Variables|/Game/UltimateFPSAnimationsKIT/Demo/PlayerMannequin/BP_PlayerCharacter.BP_PlayerCharacter_C|SetIsReloading _asbp_player_character_3 false)
          (else
            (goto _label_2)))))))

(event EventHideMuzzleFlash
  ;[1 1 1] Hide/UnhideMuzzleflash
  (Rendering|Material|SetMaterial (Variables|Default|GetMuzzelFlashPlane) 0 "/Game/UltimateFPSAnimationsKIT/GunModels/Materials/M_Transparent.M_Transparent")
  (Rendering|SetVisibility (Variables|Default|GetPointLight) false false))

(event EventFire
  (bind _returnvalue (Game|GetPlayerCharacter 0))
  (bind _returnvalue_2 (Game|GetPlayerCharacter 0))
  (bind _returnvalue_3 (Game|GetPlayerCharacter 0))
  (bind _returnvalue_4 (Game|GetPlayerController 0))
  (bind _recoilpattern (Variables|Default|GetRecoilPattern))
  (bind _maxrecoilthreshold (Variables|Default|GetMaxRecoilThreshold))
  (bind _asbp_player_character (Utilities|Casting|CastToBP_PlayerCharacter _returnvalue))
  (bind _asbp_player_character_2 (Utilities|Casting|CastToBP_PlayerCharacter _returnvalue_2))
  (bind _asbp_player_character_3 (Utilities|Casting|CastToBP_PlayerCharacter _returnvalue_3))
  (bind _arms (Variables|/Game/UltimateFPSAnimationsKIT/Demo/PlayerMannequin/BP_PlayerCharacter.BP_PlayerCharacter_C|GetArms _asbp_player_character_2))
  (bind _arms_2 (Variables|/Game/UltimateFPSAnimationsKIT/Demo/PlayerMannequin/BP_PlayerCharacter.BP_PlayerCharacter_C|GetArms _asbp_player_character_3))
  (bind _returnvalue_5 (Components|SkeletalMesh|GetAnimInstance _arms_2))
  ;[1 1 1] FIre
  (if (Variables|Default|GetChamberedAmmo)
    (Variables|Default|SetChamberedAmmo false)
    (if (> (Variables|Default|GetAmmoCount) 0)
      ;[1 1 1] Recoil
      (Utilities|FlowControl|Sequence
        (:then_0
          (Utilities|FlowControl|Sequence
            (:then_0
              (Utilities|FlowControl|DoOnce false :!label _label
                (:Completed
                  (Variables|Default|SetOGControllerRotation (Pawn|GetControlRotation (Game|GetPlayerController 0) :!class /Script/Engine.Controller)))))
            (:then_1
              (Components|Timeline|SetPlayRate _recoilpattern 1.0)
              (bind (_direction _pitch _yaw) (Timeline|RecoilPattern Play)
                (:Update
                  (if (> (Variables|Default|GetAmmoCount) 0)
                    (switch Utilities|FlowControl|Switch|SwitchonETimelineDirection _direction
                      (:Forward
                        (Class|PlayerController|AddPitchInput _returnvalue_4 _pitch)
                        (Class|PlayerController|AddYawInput _returnvalue_4 _yaw))
                      (:Backward
                        (Utilities|FlowControl|Sequence
                          (:then_0
                            (Utilities|FlowControl|DoOnce false :!label _label_2
                              (:Completed
                                (Variables|Default|SetPostRecoilRotation (Pawn|GetControlRotation (Game|GetPlayerController 0) :!class /Script/Engine.Controller)))))
                          (:then_1
                            (Class|PlayerController|AddPitchInput _returnvalue_4 (* _pitch -8.0 (select (> (Math|Float|Absolute(Float) (.Pitch (Math|Rotator|BreakRotator (Math|Rotator|Delta(Rotator) (Variables|Default|GetOGControllerRotation) (Variables|Default|GetPostRecoilRotation))))) _maxrecoilthreshold) (Math|Float|MapRangeClamped (Math|Float|Absolute(Float) (.Pitch (Math|Rotator|BreakRotator (Math|Rotator|Delta(Rotator) (Variables|Default|GetOGControllerRotation) (Variables|Default|GetPostRecoilRotation))))) _maxrecoilthreshold 3e+01 1.0 0.0) (Math|Float|MapRangeClamped (Math|Float|Absolute(Float) (.Pitch (Math|Rotator|BreakRotator (Math|Rotator|Delta(Rotator) (Variables|Default|GetOGControllerRotation) (Variables|Default|GetPostRecoilRotation))))) 0.0 _maxrecoilthreshold 0.0 1.0))))
                            (Class|PlayerController|AddYawInput _returnvalue_4 (* _yaw -1.0 (select (> (Math|Float|Absolute(Float) (.Pitch (Math|Rotator|BreakRotator (Math|Rotator|Delta(Rotator) (Variables|Default|GetOGControllerRotation) (Variables|Default|GetPostRecoilRotation))))) _maxrecoilthreshold) (Math|Float|MapRangeClamped (Math|Float|Absolute(Float) (.Pitch (Math|Rotator|BreakRotator (Math|Rotator|Delta(Rotator) (Variables|Default|GetOGControllerRotation) (Variables|Default|GetPostRecoilRotation))))) _maxrecoilthreshold 3e+01 1.0 0.0) (Math|Float|MapRangeClamped (Math|Float|Absolute(Float) (.Pitch (Math|Rotator|BreakRotator (Math|Rotator|Delta(Rotator) (Variables|Default|GetOGControllerRotation) (Variables|Default|GetPostRecoilRotation))))) 0.0 _maxrecoilthreshold 0.0 1.0))))))))))
                (:Finished
                  (switch Utilities|FlowControl|Switch|SwitchonETimelineDirection _direction
                    (:Backward
                      (Utilities|FlowControl|Sequence
                        (:then_0
                          (goto _label Reset))
                        (:then_1
                          (goto _label_2 Reset))))))))))
        (:then_1
          (CallFunction|AmmoCheck)
          (Utilities|FlowControl|Sequence
            (:then_0
              (bind (_muzzlelocation _impactpoint _projectilerotation) (CallFunction|LineTrace))
              (bind _returnvalue_6 (CallFunction|SpawnBulletProjectile _muzzlelocation _impactpoint _impactpoint _projectilerotation))
              (Game|SpawnActorfromClass "/Game/UltimateFPSAnimationsKIT/Gun_Blueprints/BP_Bullet.BP_Bullet_C" _returnvalue_6 "AdjustIfPossibleButAlwaysSpawn" 0 0))
            (:then_1
              (bind (_muzzlelocation_2 _impactpoint_2 _projectilerotation_2) (CallFunction|LineTrace))
              (bind _returnvalue_7 (CallFunction|SpawnBulletProjectile _muzzlelocation_2 _impactpoint_2 _impactpoint_2 _projectilerotation_2))
              (Game|SpawnActorfromClass "/Game/UltimateFPSAnimationsKIT/Gun_Blueprints/BP_Bullet.BP_Bullet_C" _returnvalue_7 "AdjustIfPossibleButAlwaysSpawn" 0 0))
            (:then_2
              (bind (_muzzlelocation_3 _impactpoint_3 _projectilerotation_3) (CallFunction|LineTrace))
              (bind _returnvalue_8 (CallFunction|SpawnBulletProjectile _muzzlelocation_3 _impactpoint_3 _impactpoint_3 _projectilerotation_3))
              (Game|SpawnActorfromClass "/Game/UltimateFPSAnimationsKIT/Gun_Blueprints/BP_Bullet.BP_Bullet_C" _returnvalue_8 "AdjustIfPossibleButAlwaysSpawn" 0 0))
            (:then_3
              (bind (_muzzlelocation_4 _impactpoint_4 _projectilerotation_4) (CallFunction|LineTrace))
              (bind _returnvalue_9 (CallFunction|SpawnBulletProjectile _muzzlelocation_4 _impactpoint_4 _impactpoint_4 _projectilerotation_4))
              (Game|SpawnActorfromClass "/Game/UltimateFPSAnimationsKIT/Gun_Blueprints/BP_Bullet.BP_Bullet_C" _returnvalue_9 "AdjustIfPossibleButAlwaysSpawn" 0 0))
            (:then_4
              (bind (_muzzlelocation_5 _impactpoint_5 _projectilerotation_5) (CallFunction|LineTrace))
              (bind _returnvalue_10 (CallFunction|SpawnBulletProjectile _muzzlelocation_5 _impactpoint_5 _impactpoint_5 _projectilerotation_5))
              (Game|SpawnActorfromClass "/Game/UltimateFPSAnimationsKIT/Gun_Blueprints/BP_Bullet.BP_Bullet_C" _returnvalue_10 "AdjustIfPossibleButAlwaysSpawn" 0 0))
            (:then_6
              (if (Variables|/Game/UltimateFPSAnimationsKIT/Demo/PlayerMannequin/BP_PlayerCharacter.BP_PlayerCharacter_C|GetAimDownSight _asbp_player_character_2)
                (Animation|Montage|PlayMontage _arms "/Game/UltimateFPSAnimationsKIT/Animations/Arms_Montages/SHOTGUN4_arms_fire_ads_Montage.SHOTGUN4_arms_fire_ads_Montage"
                  (:then
                    _))
                (else
                  (Animation|Montage|PlayMontage _arms "/Game/UltimateFPSAnimationsKIT/Animations/Arms_Montages/SHOTGUN4_arms_fire_Montage.SHOTGUN4_arms_fire_Montage"
                    (:then
                      _))))
              (Utilities|MuzzleFlash)
              (if (not (Variables|/Game/UltimateFPSAnimationsKIT/Demo/PlayerMannequin/BP_PlayerCharacter.BP_PlayerCharacter_C|GetAimDownSight _asbp_player_character))
                (Default|IncreaseSpread _asbp_player_character 1.0)))))
        (:then_2
          (Utilities|FlowControl|Delay 0.1)
          (Components|Timeline|SetPlayRate _recoilpattern 8.0)
          (Timeline|RecoilPattern Reverse)))
      (else
        (Audio|PlaySound2D "/Game/UltimateFPSAnimationsKIT/SoundFX/dryfire.dryfire" 1.0 1.0 0.0 0 0)))
    (else
      ;[1 1 1] Chamber New Round
      (if (> (Variables|Default|GetAmmoCount) 0)
        (Variables|/Game/UltimateFPSAnimationsKIT/Demo/PlayerMannequin/BP_PlayerCharacter.BP_PlayerCharacter_C|SetIsReloading _asbp_player_character_3 true)
        (if (Variables|/Game/UltimateFPSAnimationsKIT/Demo/PlayerMannequin/BP_PlayerCharacter.BP_PlayerCharacter_C|GetAimDownSight _asbp_player_character_3)
          (bind _returnvalue_11 (Animation|Montage|MontagePlay _returnvalue_5 "/Game/UltimateFPSAnimationsKIT/Animations/Arms_Montages/SHOTGUN4_arms_chamber_ads_Montage.SHOTGUN4_arms_chamber_ads_Montage" 1.0 "MontageLength" 0.0 true))
          (Components|Animation|PlayAnimation (Variables|Default|GetPrimaryWeapon) "/Game/UltimateFPSAnimationsKIT/Animations/Gun/SHOTGUN4_gun_chamber.SHOTGUN4_gun_chamber" false)
          (Utilities|FlowControl|Sequence
            (:then_0
              (Utilities|FlowControl|Delay _returnvalue_11)
              (Variables|Default|SetChamberedAmmo true)
              (Variables|/Game/UltimateFPSAnimationsKIT/Demo/PlayerMannequin/BP_PlayerCharacter.BP_PlayerCharacter_C|SetIsReloading _asbp_player_character_3 false))
            (:then_1
              (Utilities|FlowControl|Delay 0.2)
              (Utilities|EjectShell)))
          (else
            (bind _returnvalue_12 (Animation|Montage|MontagePlay _returnvalue_5 "/Game/UltimateFPSAnimationsKIT/Animations/Arms_Montages/SHOTGUN4_arms_chamber_Montage.SHOTGUN4_arms_chamber_Montage" 1.0 "MontageLength" 0.0 true))
            (Components|Animation|PlayAnimation (Variables|Default|GetPrimaryWeapon) "/Game/UltimateFPSAnimationsKIT/Animations/Gun/SHOTGUN4_gun_chamber.SHOTGUN4_gun_chamber" false)
            (Utilities|FlowControl|Sequence
              (:then_0
                (Utilities|FlowControl|Delay _returnvalue_12)
                (Variables|Default|SetChamberedAmmo true)
                (Variables|/Game/UltimateFPSAnimationsKIT/Demo/PlayerMannequin/BP_PlayerCharacter.BP_PlayerCharacter_C|SetIsReloading _asbp_player_character_3 false))
              (:then_1
                (Utilities|FlowControl|Delay 0.2)
                (Utilities|EjectShell)))))))))

(event EventUnhideMuzzleFlash
  ;[1 1 1] Hide/UnhideMuzzleflash
  (Rendering|Material|SetMaterial (Variables|Default|GetMuzzelFlashPlane) 0 "/Game/UltimateFPSAnimationsKIT/TexturesAndMats/M_MuzzleFlash.M_MuzzleFlash")
  (Rendering|SetVisibility (Variables|Default|GetPointLight) true false))

(event EventEquipe
  (bind _returnvalue (Game|GetPlayerCharacter 0))
  (bind _asbp_player_character (Utilities|Casting|CastToBP_PlayerCharacter _returnvalue))
  ;[1 1 1] Equipe
  (Animation|Montage|MontagePlay (Components|SkeletalMesh|GetAnimInstance (Variables|/Game/UltimateFPSAnimationsKIT/Demo/PlayerMannequin/BP_PlayerCharacter.BP_PlayerCharacter_C|GetArms _asbp_player_character)) "/Game/UltimateFPSAnimationsKIT/Animations/Arms_Montages/SHOTGUN4_arms_equipe_Montage.SHOTGUN4_arms_equipe_Montage" 1.0 "MontageLength" 0.0 true)
  (Components|Animation|PlayAnimation (Variables|Default|GetPrimaryWeapon) "/Game/UltimateFPSAnimationsKIT/Animations/Gun/SHOTGUN4_gun_equipe.SHOTGUN4_gun_equipe" false)
  (Variables|/Game/UltimateFPSAnimationsKIT/Demo/PlayerMannequin/BP_PlayerCharacter.BP_PlayerCharacter_C|SetKnifeActive _asbp_player_character false))

(event EventBeginPlay
  ;[1 1 1] Hide Bullets
  (CallFunction|HideBullets))

(fn ConstructionScript
  (|CallParentFunction)
  (Variables|Default|SetMaxAmmo 10)
  (Variables|Default|SetAmmoCount 10)
  (Variables|Default|SetReloadTime 2.0)
  (Variables|Default|SetBulletSpread 5e+02)
  (Variables|Default|SetName "NewEnumerator12")
  (Variables|Default|SetVariableMode false)
  (Variables|Default|SetIsShotgun true))

(fn AmmoCheck
  (Math|Integer|DecrementInt (Variables|Default|GetAmmoCount)
    (:%20%20
      (if (not (Variables|/Game/UltimateFPSAnimationsKIT/Demo/PlayerMannequin/BP_PlayerCharacter.BP_PlayerCharacter_C|GetIsReloading (.AsBP%20Player%20Character (Utilities|Casting|CastToBP_PlayerCharacter (Game|GetPlayerCharacter 0)))))
        (Components|Animation|PlayAnimation (Variables|Default|GetPrimaryWeapon) "/Game/UltimateFPSAnimationsKIT/Animations/Gun/SHOTGUN4_gun_fire.SHOTGUN4_gun_fire" false)))))

(fn LineTrace
  (bind _returnvalue (Game|GetPlayerCharacter 0))
  (bind _bulletspread (Variables|Default|GetBulletSpread))
  (bind _muzzle (Variables|Default|GetMuzzle))
  (bind _returnvalue_2 (Transformation|GetWorldLocation _muzzle))
  (bind _asbp_player_character (Utilities|Casting|CastToBP_PlayerCharacter _returnvalue))
  (bind _returnvalue_3 (* _bulletspread -1.0))
  (bind _playercamera (Variables|/Game/UltimateFPSAnimationsKIT/Demo/PlayerMannequin/BP_PlayerCharacter.BP_PlayerCharacter_C|GetPlayerCamera _asbp_player_character))
  (bind _returnvalue_4 (Transformation|GetWorldLocation _playercamera))
  (bind _outhit (Collision|LineTraceByChannel _returnvalue_4 (+ (+ (* (Math|Vector|GetForwardVector _playercamera) 2e+04) _returnvalue_4) (Math|Vector|MakeVector (Math|Random|RandomFloatinRange _returnvalue_3 _bulletspread) (Math|Random|RandomFloatinRange _returnvalue_3 _bulletspread) (Math|Random|RandomFloatinRange _returnvalue_3 _bulletspread))) "TraceTypeQuery1" false 0 "None")) ; CameraLineTrace
  (Collision|LineTraceByChannel _returnvalue_2 (.ImpactPoint (Collision|BreakHitResult _outhit)) "TraceTypeQuery1" false 0 "None" true "(R=0.000000,G=1.000000,B=0.110935,A=1.000000)") ; MuzzleLineTrace
  (return _returnvalue_2 (.ImpactPoint (Collision|BreakHitResult _outhit)) (Math|Rotator|FindLookatRotation (.TraceStart (Collision|BreakHitResult _outhit)) (.TraceEnd (Collision|BreakHitResult _outhit)))))

(fn SpawnBulletProjectile
  (params (MuzzleLocation :type Vector) (ImpactPoint :type Vector) (SpawnTransformLocation :type Vector) (ProjectileRotation :type Rotator))
  (Game|SpawnActorfromClass "/Game/UltimateFPSAnimationsKIT/Gun_Blueprints/BP_BulletDecal.BP_BulletDecal_C" (Math|Transform|MakeTransform SpawnTransformLocation (Math|Conversions|RotationFromXVector ImpactPoint) "0.020000,0.020000,0.020000") "Undefined" 0 0)
  (return (Math|Transform|MakeTransform MuzzleLocation ProjectileRotation "0.080000,0.080000,0.080000")))

(fn HideBullets
  (Components|SkinnedMesh|HideBonebyName (Variables|Default|GetPrimaryWeapon) "bullet" "PBO_None"))

(fn UnHideBullets
  (Components|SkinnedMesh|UnHideBonebyName (Variables|Default|GetPrimaryWeapon) "bullet"))