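; Gameplay ability that fires a weapon: one shot when WeaponMode is true, otherwise automatic fire through a Gate and RetriggerableDelay loop until the ability ends.
; Each shot checks ammo, playing a dry-fire sound when empty, then decrements it and line-traces from the WeaponBase to spawn a bullet and impact decal.
; Arms montages follow aim-down-sight state, gun animation is skipped while reloading, and hip fire increases spread.
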(event Ability|EventActivateAbility
  ;[1 1 1] Fire
  (if (Variables|Default|GetWeaponMode)
    (Utilities|FlowControl|Sequence
      (:then_0
        (bind _asweapon_base (Utilities|Casting|CastToWeaponBase (Ability|GetOwningActorfromActorInfo) :!label _label))
        (if (> (.AmmoCount (Utilities|Struct|BreakWeaponData (Variables|/Script/WeaponSystem.WeaponBase|GetWeaponData _asweapon_base))) 0)
          (CallFunction|AmmoCheck)
          (bind _asweapon_base_2 (Utilities|Casting|CastToWeaponBase (Ability|GetOwningActorfromActorInfo)))
          (bind (_outmuzzlelocation _outimactpoint _projectilerotation) (Class|WeaponBase|LineTrace _asweapon_base_2))
          (CallFunction|SpawnProjectile _outmuzzlelocation _outimactpoint _outimactpoint _projectilerotation)
          (bind _returnvalue (Class|WeaponBase|GetOwningCharacter _asweapon_base_2))
          (bind _astoy_fps_character (Utilities|Casting|CastToToyFpsCharacter _returnvalue))
          (if (Variables|/Script/ToyFPS.ToyFpsCharacter|GetbAimDownSight _astoy_fps_character)
            (Animation|Montage|PlayMontage (Variables|/Script/ToyFPS.ToyFpsCharacter|GetArmsMeshComponent _astoy_fps_character) "/Game/UltimateFPSAnimationsKIT/Animations/Arms_Montages/RIFLE5_arms_fire_ads_Montage.RIFLE5_arms_fire_ads_Montage"
              (:then
                _))
            (else
              (Animation|Montage|PlayMontage (Variables|/Script/ToyFPS.ToyFpsCharacter|GetArmsMeshComponent _astoy_fps_character) "/Game/UltimateFPSAnimationsKIT/Animations/Arms_Montages/RIFLE5_arms_fire_Montage.RIFLE5_arms_fire_Montage"
                (:then
                  _))))
          (bind _astoy_fps_character_2 (Utilities|Casting|CastToToyFpsCharacter (Game|GetPlayerCharacter 0)))
          (if (not (Variables|/Script/ToyFPS.ToyFpsCharacter|GetbAimDownSight _astoy_fps_character_2))
            (Class|ToyFpsCharacter|IncreaseSpread _astoy_fps_character_2 0.06))
          (else
            (Audio|PlaySound2D "/Game/UltimateFPSAnimationsKIT/SoundFX/dryfire.dryfire" 1.0 1.0 0.0 0 0))))
      (:then_1
        (Utilities|FlowControl|Delay 0.1)))
    (else
      (Utilities|FlowControl|Sequence
        (:then_0
          (goto _label_2 Open))
        (:then_1
          (Utilities|FlowControl|Gate true :!label _label_2
            (:Exit
              (Utilities|FlowControl|Sequence
                (:then_0
                  (goto _label))
                (:then_1
                  (Utilities|FlowControl|RetriggerableDelay 0.12)
                  (goto _label_2))))))))))

(event Ability|EventOnEndAbility
  (params (bWasCancelled :type Boolean))
  ;[1 1 1] Fire
  (Utilities|FlowControl|Sequence
    (:then_0
      (Utilities|FlowControl|Gate true) ; enters at Close
    )))

(fn AmmoCheck
  (bind _asweapon_base (Utilities|Casting|CastToWeaponBase (Ability|GetOwningActorfromActorInfo)))
  (Math|Integer|DecrementInt (.AmmoCount (Utilities|Struct|BreakWeaponData (Variables|/Script/WeaponSystem.WeaponBase|GetWeaponData _asweapon_base)))
    (:%20%20
      (bind _astoy_fps_character (Utilities|Casting|CastToToyFpsCharacter (Game|GetPlayerCharacter 0)))
      (if (not (Variables|/Script/ToyFPS.ToyFpsCharacter|GetbReloading _astoy_fps_character))
        (bind _asweapon_base_2 (Utilities|Casting|CastToWeaponBase (Ability|GetOwningActorfromActorInfo)))
        (Components|Animation|PlayAnimation (Variables|/Script/WeaponSystem.WeaponBase|GetPrimaryWeapon _asweapon_base_2) "/Game/UltimateFPSAnimationsKIT/Animations/Gun/RIFLE5_gun_fire.RIFLE5_gun_fire" false)))))

(fn SpawnProjectile
  (params (MuzzleLocation :type Vector) (ImpactPoint :type Vector) (SpawnTransformLocation :type Vector) (ProjectileRotation :type Rotator))
  (Game|SpawnActorfromClass "/Game/UltimateFPSAnimationsKIT/Gun_Blueprints/BP_BulletDecal.BP_BulletDecal_C" (Math|Transform|MakeTransform SpawnTransformLocation (Math|Conversions|RotationFromXVector ImpactPoint) "0.020000,0.020000,0.020000") "Undefined" 0 0)
  (Game|SpawnActorfromClass "/Game/UltimateFPSAnimationsKIT/Gun_Blueprints/BP_Bullet.BP_Bullet_C" (Math|Transform|MakeTransform MuzzleLocation ProjectileRotation "0.080000,0.080000,0.080000") "Undefined" 0 0)
  (return))