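; BP_TestTarget is a damage test target actor that displays its health on a text render component.
; The construction script writes the Health value into the text.
; On AnyDamage it refreshes the health readout, or shows red "Dead" text when the Dead flag is set.
; The graph only reads Health and Dead and does not modify either value.
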(event EventBeginPlay)

(event Collision|EventActorBeginOverlap
  (params (OtherActor :type Actor%20Object%20Reference)))

(event EventTick
  (params (DeltaSeconds :type Float%20%28single-precision%29)))

(event Game|Damage|EventAnyDamage
  (params (Damage :type Float%20%28single-precision%29) (DamageType :type Damage%20Type%20Object%20Reference) (InstigatedBy :type Controller%20Object%20Reference) (DamageCauser :type Actor%20Object%20Reference))
  (bind _textrender (Variables|Default|GetTextRender))
  (if (Variables|Default|GetbDead)
    (Rendering|Components|TextRender|SetTextRenderColor _textrender (Math|Conversions|ToColor(LinearColor) "(R=1.000000,G=0.000000,B=0.000000,A=1.000000)"))
    (Rendering|Components|TextRender|SetText _textrender (Utilities|Text|ToText(String) "Dead"))
    (else
      (Rendering|Components|TextRender|SetText (Variables|Default|GetTextRender) (Utilities|Text|ToText(Float) (Variables|Default|GetHealth) "HalfToEven")))))

(fn ConstructionScript
  (Rendering|Components|TextRender|SetText (Variables|Default|GetTextRender) (Utilities|Text|ToText(Float) (Variables|Default|GetHealth) "HalfToEven")))