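; Gameplay ability that reloads the owning rifle when its magazine is not full.
; It picks one of four DoOnce-guarded branches by empty magazine and aim-down-sight state, playing character montages from WeaponData alongside gun animations.
; After the reload delay it refills ammo and clears Reloading, without calling EndAbility.
; Empty reloads also spawn a magazine actor at the mag socket and temporarily hide magazine and bullet bones.
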(event Ability|EventActivateAbility
  ;[1 1 1] Reload
  (bind _asweapon_base (Utilities|Casting|CastToWeaponBase (Ability|GetOwningActorfromActorInfo)))
  (bind _returnvalue (Class|WeaponBase|GetOwningCharacter _asweapon_base))
  (if (< (.AmmoCount (Utilities|Struct|BreakWeaponData (Variables|/Script/WeaponSystem.WeaponBase|GetWeaponData _asweapon_base))) (.MaxAmmo (Utilities|Struct|BreakWeaponData (Variables|/Script/WeaponSystem.WeaponBase|GetWeaponData _asweapon_base))))
    (if (< (.AmmoCount (Utilities|Struct|BreakWeaponData (Variables|/Script/WeaponSystem.WeaponBase|GetWeaponData _asweapon_base))) 1)
      (if (Variables|/Script/ToyFPS.ToyFpsCharacter|GetbAimDownSight _returnvalue)
        (Utilities|FlowControl|DoOnce false :!label _label
          (:Completed
            (Variables|/Script/ToyFPS.ToyFpsCharacter|SetbReloading _returnvalue true)
            (Animation|Montage|MontagePlay (Components|SkeletalMesh|GetAnimInstance (Variables|/Script/ToyFPS.ToyFpsCharacter|GetArmsMeshComponent _returnvalue)) (.AnimMontage_AdsEmptyWeaponReload (Utilities|Struct|BreakWeaponData (Variables|/Script/WeaponSystem.WeaponBase|GetWeaponData _asweapon_base))) 1.0 "MontageLength" 0.0 true)
            (Utilities|FlowControl|Sequence
              (:then_0
                (Components|Animation|PlayAnimation (Variables|/Script/WeaponSystem.WeaponBase|GetPrimaryWeapon _asweapon_base) "/Game/UltimateFPSAnimationsKIT/Animations/Gun/RIFLE5_gun_reload_empty.RIFLE5_gun_reload_empty" false)
                (Utilities|FlowControl|Delay (.ReloadTime (Utilities|Struct|BreakWeaponData (Variables|/Script/WeaponSystem.WeaponBase|GetWeaponData _asweapon_base))))
                (Class|WeaponBase|ReloadAmmo _asweapon_base)
                (Variables|/Script/ToyFPS.ToyFpsCharacter|SetbReloading _returnvalue false)
                (goto _label Reset))
              (:then_1
                _))))
        (else
          (Utilities|FlowControl|DoOnce false :!label _label_2
            (:Completed
              (Variables|/Script/ToyFPS.ToyFpsCharacter|SetbReloading _returnvalue true)
              (CallFunction|HideAmmo)
              (Animation|Montage|MontagePlay (Components|SkeletalMesh|GetAnimInstance (Variables|/Script/ToyFPS.ToyFpsCharacter|GetArmsMeshComponent _returnvalue)) (.AnimMontage_EmptyWeaponReload (Utilities|Struct|BreakWeaponData (Variables|/Script/WeaponSystem.WeaponBase|GetWeaponData _asweapon_base))) 1.0 "MontageLength" 0.0 true)
              (Utilities|FlowControl|Sequence
                (:then_0
                  (Components|Animation|PlayAnimation (Variables|/Script/WeaponSystem.WeaponBase|GetPrimaryWeapon _asweapon_base) "/Game/UltimateFPSAnimationsKIT/Animations/Gun/RIFLE5_gun_reload_empty.RIFLE5_gun_reload_empty" false)
                  (Utilities|FlowControl|Delay (.ReloadTime (Utilities|Struct|BreakWeaponData (Variables|/Script/WeaponSystem.WeaponBase|GetWeaponData _asweapon_base))))
                  (Class|WeaponBase|ReloadAmmo _asweapon_base)
                  (Variables|/Script/ToyFPS.ToyFpsCharacter|SetbReloading _returnvalue false)
                  (goto _label_2 Reset))
                (:then_1
                  _))))))
      ;;[1 1 1] Mag Spawn
      (Utilities|FlowControl|Sequence
        (:then_0
          (Utilities|FlowControl|Delay 0.8)
          (Game|SpawnActorfromClass "/Game/UltimateFPSAnimationsKIT/MagDrops/BP_Mag_Rifle5.BP_Mag_Rifle5_C" (Transformation|GetSocketTransform (Variables|/Script/WeaponSystem.WeaponBase|GetPrimaryWeapon _asweapon_base) "magSocket" "RTS_World") "Undefined" "OverrideRootScale" 0 0))
        (:then_1
          ;;[1 1 1] Hiding Mag
          (Utilities|FlowControl|Delay 0.2)
          (Components|SkinnedMesh|HideBonebyName (Variables|/Script/WeaponSystem.WeaponBase|GetPrimaryWeapon _asweapon_base) "mag" "PBO_None")
          (Components|SkinnedMesh|HideBonebyName (Variables|/Script/WeaponSystem.WeaponBase|GetPrimaryWeapon _asweapon_base) "bullet" "PBO_None")
          (Components|SkinnedMesh|HideBonebyName (Variables|/Script/WeaponSystem.WeaponBase|GetPrimaryWeapon _asweapon_base) "bullets" "PBO_None")
          (Utilities|FlowControl|Delay 0.8)
          (Components|SkinnedMesh|UnHideBonebyName (Variables|/Script/WeaponSystem.WeaponBase|GetPrimaryWeapon _asweapon_base) "mag")
          (Components|SkinnedMesh|UnHideBonebyName (Variables|/Script/WeaponSystem.WeaponBase|GetPrimaryWeapon _asweapon_base) "bullet")
          (Components|SkinnedMesh|UnHideBonebyName (Variables|/Script/WeaponSystem.WeaponBase|GetPrimaryWeapon _asweapon_base) "bullets")))
      (elif (Variables|/Script/ToyFPS.ToyFpsCharacter|GetbAimDownSight _returnvalue)
        (Utilities|FlowControl|DoOnce false :!label _label_3
          (:Completed
            (Variables|/Script/ToyFPS.ToyFpsCharacter|SetbReloading _returnvalue true)
            (Animation|Montage|MontagePlay (Components|SkeletalMesh|GetAnimInstance (Variables|/Script/Engine.Character|GetMesh _returnvalue)) (.AnimMontage_AdsWeaponReload (Utilities|Struct|BreakWeaponData (Variables|/Script/WeaponSystem.WeaponBase|GetWeaponData _asweapon_base))) 1.0 "MontageLength" 0.0 true)
            (Components|Animation|PlayAnimation (Variables|/Script/WeaponSystem.WeaponBase|GetPrimaryWeapon _asweapon_base) "/Game/UltimateFPSAnimationsKIT/Animations/Gun/RIFLE5_gun_reload.RIFLE5_gun_reload" false)
            (Utilities|FlowControl|Delay (.ReloadTime (Utilities|Struct|BreakWeaponData (Variables|/Script/WeaponSystem.WeaponBase|GetWeaponData _asweapon_base))))
            (Class|WeaponBase|ReloadAmmo _asweapon_base)
            (Variables|/Script/ToyFPS.ToyFpsCharacter|SetbReloading _returnvalue false)
            (goto _label_3 Reset)))
        (else
          (Utilities|FlowControl|DoOnce false :!label _label_4
            (:Completed
              (Variables|/Script/ToyFPS.ToyFpsCharacter|SetbReloading _returnvalue true)
              (Animation|Montage|MontagePlay (Components|SkeletalMesh|GetAnimInstance (Variables|/Script/ToyFPS.ToyFpsCharacter|GetArmsMeshComponent _returnvalue)) (.AnimMontage_WeaponReload (Utilities|Struct|BreakWeaponData (Variables|/Script/WeaponSystem.WeaponBase|GetWeaponData _asweapon_base))) 1.0 "MontageLength" 0.0 true)
              (Components|Animation|PlayAnimation (Variables|/Script/WeaponSystem.WeaponBase|GetPrimaryWeapon _asweapon_base) "/Game/UltimateFPSAnimationsKIT/Animations/Gun/RIFLE5_gun_reload.RIFLE5_gun_reload" false)
              (Utilities|FlowControl|Delay (.ReloadTime (Utilities|Struct|BreakWeaponData (Variables|/Script/WeaponSystem.WeaponBase|GetWeaponData _asweapon_base))))
              (Class|WeaponBase|ReloadAmmo _asweapon_base)
              (Variables|/Script/ToyFPS.ToyFpsCharacter|SetbReloading _returnvalue false)
              (goto _label_4 Reset))))))))

(event Ability|EventOnEndAbility
  (params (bWasCancelled :type Boolean)))

(fn HideAmmo
  (bind _asweapon_base (Utilities|Casting|CastToWeaponBase (Ability|GetOwningActorfromActorInfo)))
  (Components|SkinnedMesh|HideBonebyName (Variables|/Script/WeaponSystem.WeaponBase|GetPrimaryWeapon _asweapon_base) "bullet" "PBO_None")
  (Components|SkinnedMesh|HideBonebyName (Variables|/Script/WeaponSystem.WeaponBase|GetPrimaryWeapon _asweapon_base) "bullets" "PBO_None"))